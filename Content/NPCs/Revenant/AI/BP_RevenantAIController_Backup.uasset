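; AI controller for the Revenant NPC, apparently a backup copy, that reacts to perceiving the player.
; When AI Perception senses a BP_ThirdPersonCharacter, it stores it as TargetPlayer and changes the controlled Revenant's CurrentState.
; A failed-sense update clears TargetPlayer but leaves the Revenant's state untouched.
; UpdateBehaviour is an unfinished stub holding only an authority switch with nothing wired after it.
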(event OnTargetPerceptionUpdated(AIPerception)
  (params (Actor :type Actor%20Object%20Reference) (Stimulus :type AI%20Stimulus%20Structure))
  (bind _bsuccessfullysensed (Utilities|Struct|BreakAIStimulus Stimulus))
  (if _bsuccessfullysensed
    (bind _asbp_third_person_character (Utilities|Casting|CastToBP_ThirdPersonCharacter Actor))
    (Variables|Default|SettargetPlayer _asbp_third_person_character)
    (if _bsuccessfullysensed
      (bind _asbp_revenant (Utilities|Casting|CastToBP_Revenant (Pawn|GetControlledPawn)))
      (Variables|/Game/NPCs/Revenant/Character/BP_Revenant.BP_Revenant_C|SetcurrentState _asbp_revenant "NewEnumerator1"))
    (else
      (Variables|Default|SettargetPlayer 0))))

(event Custom|UpdateBehaviour
  (Networking|SwitchHasAuthority))

(event EventBeginPlay)

(event EventTick
  (params (DeltaSeconds :type Float%20%28single-precision%29)))

(fn ConstructionScript)