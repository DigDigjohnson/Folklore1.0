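; AI controller for the Revenant NPC, an early scaffold of a state machine with wandering, stalking, investigating, hunting, exorcism and banished states.
; Think picks a state from target validity and visibility, and ChangeState fires its Enter event once.
; Only Wandering acts, chaining AIMoveTo between random reachable points.
; Perception, targeting and update functions are stubs; initialization and the Think timer are disconnected, while possession starts a separate looping timer.
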(event Custom|EnterWandering
  (bind _wanderingradius (Variables|AI|Config|GetwanderingRadius))
  (bind _controlledrevenant (Variables|References|GetcontrolledRevenant))
  (bind _returnvalue (Transformation|GetActorLocation _controlledrevenant))
  (bind (_randomlocation _returnvalue_2) (AI|Navigation|GetRandomReachablePointinRadius _returnvalue _wanderingradius 0 0))
  ;[0.15 0.15 0.15 0.5] Enter States
  (if _returnvalue_2
    (AI|AIMoveTo (Variables|References|GetcontrolledRevenant) _randomlocation 0 1e+02 true
      (:OnSuccess
        (CallFunction|EnterWandering)))))

(event Custom|EnterStalking
  ;[0.15 0.15 0.15 0.5] Enter States
)

(event Custom|EnterInvestigating
  ;[0.15 0.15 0.15 0.5] Enter States
)

(event Custom|EnterHunting
  ;[0.15 0.15 0.15 0.5] Enter States
)

(event Custom|EnterExorcism
  ;[0.15 0.15 0.15 0.5] Enter States
)

(event Custom|EnterBanished
  ;[0.15 0.15 0.15 0.5] Enter States
)

(event EventBeginPlay
  ;[0.15 0.15 0.15 0.5] Engine Events
)

(event EventPossess
  (params (PossessedPawn :type Pawn%20Object%20Reference))
  ;[0.15 0.15 0.15 0.5] Engine Events
  (bind _asbp_revenant (Utilities|Casting|CastToBP_Revenant PossessedPawn))
  (Variables|References|SetcontrolledRevenant _asbp_revenant)
  (Utilities|Time|SetTimerbyEvent (EventDispatchers|CreateEvent :!event Think) 0.2 true))

(fn ConstructionScript)

(fn InitializeAI
  (Variables|state|SetcurrentState "NewEnumerator0")
  (Variables|state|SetlastState "NewEnumerator0")
  (Variables|state|SetcurrentStateStarted false))

(fn ChooseTarget)

(fn StopMove
  (AI|Navigation|StopMovement))

(fn Think
  ;[0.15 0.15 0.15 0.5] Decide qual estado a IA deve assumir
  (AI|Brain|UpdatePerception)
  (AI|Brain|ChooseTarget)
  (Utilities|IsValid (Variables|AI|Target|GetcurrentTarget)
    (:Is%20Valid
      (if (Variables|AI|Target|GetcanSeeTarget)
        (AI|Brain|ChangeState "NewEnumerator1")
        (else
          (AI|Brain|ChangeState "NewEnumerator5"))))
    (:Is%20Not%20Valid
      (AI|Brain|ChangeState "NewEnumerator0"))))

(fn ExecuteCurrentState
  (if (not (Variables|state|GetcurrentStateStarted))
    (Variables|state|SetcurrentStateStarted true)
    (switch Utilities|FlowControl|Switch|SwitchonE_RevenantStates (Variables|state|GetcurrentState)
      (:NewEnumerator0
        (CallFunction|EnterWandering))
      (:NewEnumerator1
        (CallFunction|EnterStalking))
      (:NewEnumerator5
        (CallFunction|EnterInvestigating))
      (:NewEnumerator2
        (CallFunction|EnterHunting))
      (:NewEnumerator3
        (CallFunction|EnterExorcism))
      (:NewEnumerator4
        (CallFunction|EnterBanished)))))

(fn ChangeState
  (params (newState :type E_RevenantStates%20Enum :default "NewEnumerator0"))
  ;[0.15 0.15 0.15 0.5] Realiza a troca entre estados
  (if (not (Utilities|Enum|Equal(Enum) newState (Variables|state|GetcurrentState)))
    (Variables|state|SetlastState (Variables|state|GetcurrentState))
    (Variables|state|SetcurrentState newState)
    (Variables|state|SetcurrentStateStarted false)
    (CallFunction|ExecuteCurrentState)))

(fn UpdateCurrentState
  ;[0.15 0.15 0.15 0.5] Atualiza continuamente o estado atual
  (switch Utilities|FlowControl|Switch|SwitchonE_RevenantStates (Variables|state|GetcurrentState)
    (:NewEnumerator0
      (AI|States|Update|UpdateWandering))
    (:NewEnumerator1
      (AI|States|Update|UpdateStalking))
    (:NewEnumerator5
      (AI|States|Update|UpdateInvestigating))
    (:NewEnumerator2
      (AI|States|Update|UpdateHunting))
    (:NewEnumerator3
      (AI|States|Update|UpdateExorcism))
    (:NewEnumerator4
      (AI|States|Update|UpdateBanished))))

(fn UpdateWandering)

(fn UpdateStalking)

(fn UpdateInvestigating)

(fn UpdateHunting)

(fn UpdateExorcism)

(fn UpdateBanished)

(fn UpdatePerception)